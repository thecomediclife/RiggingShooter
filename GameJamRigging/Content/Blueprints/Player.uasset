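; Player character with side-scroller style movement along the world Y axis, plus jump, crouch, aim and fire.
; A timeline yaws the actor to face its movement direction, while crouch halves walk speed and button flags track jump, crouch and aim.
; Holding aim runs a timeline that line-traces from the mouse cursor and sets a clamped SpawnPoint pitch toward the hit.
; Fire spawns a projectile ahead of SpawnPoint and plays a sound.
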(event Custom|Turn
  (params (Right :type Boolean))
  (if Right
    (bind _rotation (Timeline|Turning Play)
      (:Update
        (Transformation|SetActorRotation (Math|Rotator|MakeRotator 0.0 0.0 _rotation))))
    (else
      (Timeline|Turning Reverse))))

(event Input|ActionEvents|InputActionCrouch
  (params (Key :type Key%20Structure :default "AnyKey"))
  (bind _charactermovement (Variables|Character|GetCharacterMovement))
  (bind _charactermovement_2 (Variables|Character|GetCharacterMovement))
  (:Pressed
    (Variables|Default|SetCrouch%20Button%20Down true)
    (Variables|/Script/Engine.CharacterMovementComponent|SetMaxWalkSpeed _charactermovement_2 (/ (Variables|/Script/Engine.CharacterMovementComponent|GetMaxWalkSpeed _charactermovement_2) 2.0)))
  (:Released
    (Variables|Default|SetCrouch%20Button%20Down false)
    (Variables|/Script/Engine.CharacterMovementComponent|SetMaxWalkSpeed _charactermovement (* (Variables|/Script/Engine.CharacterMovementComponent|GetMaxWalkSpeed _charactermovement) 2.0))))

(event Input|ActionEvents|InputActionFire
  (params (Key :type Key%20Structure :default "AnyKey"))
  (bind _spawnpoint (Variables|Default|GetSpawnPoint))
  (bind _returnvalue (Transformation|GetWorldTransform _spawnpoint))
  (bind (_location _rotation _scale) (Math|Transform|BreakTransform _returnvalue))
  (:Pressed
    (Game|SpawnActorfromClass "/Game/FirstPersonBP/Blueprints/FirstPersonProjectile.FirstPersonProjectile_C" (Math|Transform|MakeTransform (+ _location (* (Math|Vector|GetForwardVector _spawnpoint) 2e+02)) _rotation _scale) "AdjustIfPossibleButDontSpawnIfColliding" 0 0) ; Spawn projectile
    (Audio|PlaySoundatLocation "/Game/FirstPerson/Audio/FirstPersonTemplateWeaponFire02.FirstPersonTemplateWeaponFire02" (Transformation|GetActorLocation)) ; Play firing sound
  ))

(event Input|ActionEvents|InputActionJump
  (params (Key :type Key%20Structure :default "AnyKey"))
  (:Pressed
    (Character|Jump)
    (Variables|Default|SetJump%20Button%20Down (Character|CanJump))
    (bind _ascharacter_movement_component (Utilities|Casting|CastToCharacterMovementComponent (Pawn|GetMovementComponent) :!label _label))
    (if (> (Math|Vector|VectorLength (Variables|/Script/Engine.MovementComponent|GetVelocity _ascharacter_movement_component)) 0.0)
      (Variables|/Script/Engine.CharacterMovementComponent|SetJumpZVelocity _ascharacter_movement_component 4e+02)
      (else
        (Variables|/Script/Engine.CharacterMovementComponent|SetJumpZVelocity _ascharacter_movement_component 4e+02))))
  (:Released
    (Character|StopJumping)
    (Variables|Default|SetJump%20Button%20Down false)
    (goto _label)))

(event Input|ActionEvents|InputActionAim
  (params (Key :type Key%20Structure :default "AnyKey"))
  (bind _returnvalue (Game|GetPlayerController 0))
  (bind (_locationx _locationy) (Game|Player|GetMousePosition _returnvalue))
  (bind (_worldlocation _worlddirection) (Class|PlayerController|DeprojectScreenPositiontoWorld _returnvalue _locationx _locationy))
  (:Pressed
    (Variables|Default|SetAimButtonDown true)
    (Timeline|Timeline_0 Play
      (:Update
        (bind (_outhit _returnvalue_2) (Collision|LineTraceForObjects _worldlocation (+ _worldlocation (* _worlddirection 2e+04)) (Utilities|Array|MakeArray "ObjectTypeQuery9") false 0 "None"))
        (if _returnvalue_2
          (Transformation|SetRelativeRotation (Variables|Default|GetSpawnPoint) (Math|Rotator|MakeRotator 0.0 (Math|Float|Clamp(Float) (* (.Pitch (Math|Rotator|BreakRotator (Math|Rotator|FindLookatRotation (Transformation|GetActorLocation) (.ImpactPoint (Collision|BreakHitResult _outhit))))) 1.0) -45.0 45.0) 9e+01) false false)))))
  (:Released
    (Variables|Default|SetAimButtonDown false)
    (Timeline|Timeline_0 Stop)))

(event Input|AxisEvents|InputAxisMoveRight
  (params (AxisValue :type Float%20%28single-precision%29))
  (Pawn|Input|AddMovementInput "0.000000,1.000000, 0" (* AxisValue (Variables|Default|GetSpeed)) false)
  (Math|Float|CompareFloat AxisValue 0.0
    (:>
      (CallFunction|Turn false))
    (:<
      (CallFunction|Turn true))))

(fn ConstructionScript)