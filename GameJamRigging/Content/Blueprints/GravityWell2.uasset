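; Gravity well actor that redirects FirstPersonProjectiles entering its sphere by hiding each one and spawning a replacement on the opposite side.
; Exit direction swings from straight through to reversed as aim strays from the center, bending along the projectile's up axis toward the well.
; SetSpline briefly shows SplineMesh at an exit transform from CalculatePassingObjects, which repeats the overlap's inline math.
; The Source check ignores projectiles the well itself spawned.
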(event OnComponentBeginOverlap(Sphere)
  (params (OtherActor :type Actor%20Object%20Reference) (OtherComp :type Primitive%20Component%20Object%20Reference) (OtherBodyIndex :type Integer) (bFromSweep :type Boolean) (SweepResult :type Hit%20Result%20Structure%20%28by%20ref%29))
  (bind _returnvalue (Transformation|GetActorLocation))
  (bind _returnvalue_2 (Transformation|GetActorLocation))
  (if (== (Utilities|GetClass OtherActor) "/Game/Blueprints/FirstPersonProjectile.FirstPersonProjectile_C")
    (bind _asfirst_person_projectile (Utilities|Casting|CastToFirstPersonProjectile OtherActor))
    (if (!= (Variables|/Game/Blueprints/FirstPersonProjectile.FirstPersonProjectile_C|GetSource _asfirst_person_projectile) self)
      (Variables|Default|SetProjectile _asfirst_person_projectile)
      (Game|SpawnActorfromClass "/Game/Blueprints/FirstPersonProjectile.FirstPersonProjectile_C" (Math|Transform|MakeTransform (+ (* (Math|Vector|Normalize (- _returnvalue_2 (Transformation|GetActorLocation (Variables|Default|GetProjectile)))) (Variables|/Script/Engine.SphereComponent|GetSphereRadius (Variables|Default|GetSphere))) _returnvalue_2) (Math|Rotator|FindLookatRotation (Transformation|GetActorLocation (Variables|Default|GetProjectile)) (+ (* (Math|Vector|Normalize (+ (* (Transformation|GetActorForwardVector (Variables|Default|GetProjectile)) (Math|Float|Lerp -1.0 1.0 (- 1.0 (Math|Float|Clamp(Float) (Class|KismetMathLibrary|InverseLerp 0.0 1.5e+02 (Math|Vector|VectorLength (- (+ (* (Transformation|GetActorForwardVector (Variables|Default|GetProjectile)) (Math|Vector|VectorLength (- (Transformation|GetActorLocation (Variables|Default|GetProjectile)) (Transformation|GetActorLocation)))) (Transformation|GetActorLocation (Variables|Default|GetProjectile))) (Transformation|GetActorLocation)))))))) (* (Transformation|GetActorUpVector (Variables|Default|GetProjectile)) (Math|Float|SelectFloat (* (Math|Float|Lerp 0.0 1.0 (Math|Float|SelectFloat (* (Math|Float|Clamp(Float) (Class|KismetMathLibrary|InverseLerp 0.0 1.5e+02 (Math|Vector|VectorLength (- (+ (* (Transformation|GetActorForwardVector (Variables|Default|GetProjectile)) (Math|Vector|VectorLength (- (Transformation|GetActorLocation (Variables|Default|GetProjectile)) (Transformation|GetActorLocation)))) (Transformation|GetActorLocation (Variables|Default|GetProjectile))) (Transformation|GetActorLocation))))) 2.0) (* (- 1.0 (Math|Float|Clamp(Float) (Class|KismetMathLibrary|InverseLerp 0.0 1.5e+02 (Math|Vector|VectorLength (- (+ (* (Transformation|GetActorForwardVector (Variables|Default|GetProjectile)) (Math|Vector|VectorLength (- (Transformation|GetActorLocation (Variables|Default|GetProjectile)) (Transformation|GetActorLocation)))) (Transformation|GetActorLocation (Variables|Default|GetProjectile))) (Transformation|GetActorLocation)))))) 2.0) (< (Math|Float|Clamp(Float) (Class|KismetMathLibrary|InverseLerp 0.0 1.5e+02 (Math|Vector|VectorLength (- (+ (* (Transformation|GetActorForwardVector (Variables|Default|GetProjectile)) (Math|Vector|VectorLength (- (Transformation|GetActorLocation (Variables|Default|GetProjectile)) (Transformation|GetActorLocation)))) (Transformation|GetActorLocation (Variables|Default|GetProjectile))) (Transformation|GetActorLocation))))) 0.5))) -1.0) (Math|Float|Lerp 0.0 1.0 (Math|Float|SelectFloat (* (Math|Float|Clamp(Float) (Class|KismetMathLibrary|InverseLerp 0.0 1.5e+02 (Math|Vector|VectorLength (- (+ (* (Transformation|GetActorForwardVector (Variables|Default|GetProjectile)) (Math|Vector|VectorLength (- (Transformation|GetActorLocation (Variables|Default|GetProjectile)) (Transformation|GetActorLocation)))) (Transformation|GetActorLocation (Variables|Default|GetProjectile))) (Transformation|GetActorLocation))))) 2.0) (* (- 1.0 (Math|Float|Clamp(Float) (Class|KismetMathLibrary|InverseLerp 0.0 1.5e+02 (Math|Vector|VectorLength (- (+ (* (Transformation|GetActorForwardVector (Variables|Default|GetProjectile)) (Math|Vector|VectorLength (- (Transformation|GetActorLocation (Variables|Default|GetProjectile)) (Transformation|GetActorLocation)))) (Transformation|GetActorLocation (Variables|Default|GetProjectile))) (Transformation|GetActorLocation)))))) 2.0) (< (Math|Float|Clamp(Float) (Class|KismetMathLibrary|InverseLerp 0.0 1.5e+02 (Math|Vector|VectorLength (- (+ (* (Transformation|GetActorForwardVector (Variables|Default|GetProjectile)) (Math|Vector|VectorLength (- (Transformation|GetActorLocation (Variables|Default|GetProjectile)) (Transformation|GetActorLocation)))) (Transformation|GetActorLocation (Variables|Default|GetProjectile))) (Transformation|GetActorLocation))))) 0.5))) (> (Math|Vector|VectorLength (- (+ (* (Transformation|GetActorUpVector (Variables|Default|GetProjectile)) 1e+02) (Transformation|GetActorLocation (Variables|Default|GetProjectile))) _returnvalue)) (Math|Vector|VectorLength (- (+ (* (Transformation|GetActorUpVector (Variables|Default|GetProjectile)) -1e+02) (Transformation|GetActorLocation (Variables|Default|GetProjectile))) _returnvalue))))))) 5e+01) (Transformation|GetActorLocation (Variables|Default|GetProjectile)))) "1.000000,1.000000,1.000000") "Undefined" 0 self 1)
      (Rendering|SetActorHiddenInGame (Variables|Default|GetProjectile) true)
      (Actor|SetLifeSpan (Variables|Default|GetProjectile) 0.1)
      (bind _asfirst_person_projectile_2 (Utilities|Casting|CastToFirstPersonProjectile (Variables|Default|GetProjectile)))
      (Variables|/Game/Blueprints/FirstPersonProjectile.FirstPersonProjectile_C|SetDisappear _asfirst_person_projectile_2 true))))

(event Custom|SetSpline
  (params (Location :type Vector) (SourceLocation :type Vector) (NewParam :type Vector))
  (Development|SetHiddeninGame (Variables|Default|GetSplineMesh) false false)
  (bind (_exitlocation _exitrotation) (CallFunction|CalculatePassingObjects Location SourceLocation NewParam))
  (Transformation|SetWorldTransform (Variables|Default|GetSplineMesh) (Math|Transform|MakeTransform _exitlocation _exitrotation) false false)
  (Utilities|FlowControl|RetriggerableDelay 0.05)
  (Development|SetHiddeninGame (Variables|Default|GetSplineMesh) true false))

(fn ConstructionScript)

(fn CalculatePassingObjects
  (params (EnterLocation :type Vector) (ForwardVector :type Vector) (UpVector :type Vector))
  (bind _returnvalue (Transformation|GetActorLocation))
  (bind _returnvalue_2 (Transformation|GetActorLocation))
  (LocalVariables|SetEnterLoc EnterLocation)
  (LocalVariables|SetFVec ForwardVector)
  (LocalVariables|SetUpVec UpVector)
  (return (+ (* (Math|Vector|Normalize (- _returnvalue_2 (LocalVariables|GetEnterLoc))) (Variables|/Script/Engine.SphereComponent|GetSphereRadius (Variables|Default|GetSphere))) _returnvalue_2) (Math|Rotator|FindLookatRotation (LocalVariables|GetEnterLoc) (+ (* (Math|Vector|Normalize (+ (* (LocalVariables|GetFVec) (Math|Float|Lerp -5e+01 5e+01 (- 1.0 (Math|Float|Clamp(Float) (Class|KismetMathLibrary|InverseLerp 0.0 1.5e+02 (Math|Vector|VectorLength (- (+ (* ForwardVector (Math|Vector|VectorLength (- (LocalVariables|GetEnterLoc) (Transformation|GetActorLocation)))) (LocalVariables|GetEnterLoc)) (Transformation|GetActorLocation)))))))) (* (LocalVariables|GetUpVec) (Math|Float|SelectFloat (* (Math|Float|Lerp 0.0 5e+01 (Math|Float|SelectFloat (* (Math|Float|Clamp(Float) (Class|KismetMathLibrary|InverseLerp 0.0 1.5e+02 (Math|Vector|VectorLength (- (+ (* ForwardVector (Math|Vector|VectorLength (- (LocalVariables|GetEnterLoc) (Transformation|GetActorLocation)))) (LocalVariables|GetEnterLoc)) (Transformation|GetActorLocation))))) 2.0) (* (- 1.0 (Math|Float|Clamp(Float) (Class|KismetMathLibrary|InverseLerp 0.0 1.5e+02 (Math|Vector|VectorLength (- (+ (* ForwardVector (Math|Vector|VectorLength (- (LocalVariables|GetEnterLoc) (Transformation|GetActorLocation)))) (LocalVariables|GetEnterLoc)) (Transformation|GetActorLocation)))))) 2.0) (< (Math|Float|Clamp(Float) (Class|KismetMathLibrary|InverseLerp 0.0 1.5e+02 (Math|Vector|VectorLength (- (+ (* ForwardVector (Math|Vector|VectorLength (- (LocalVariables|GetEnterLoc) (Transformation|GetActorLocation)))) (LocalVariables|GetEnterLoc)) (Transformation|GetActorLocation))))) 0.5))) -1.0) (Math|Float|Lerp 0.0 5e+01 (Math|Float|SelectFloat (* (Math|Float|Clamp(Float) (Class|KismetMathLibrary|InverseLerp 0.0 1.5e+02 (Math|Vector|VectorLength (- (+ (* ForwardVector (Math|Vector|VectorLength (- (LocalVariables|GetEnterLoc) (Transformation|GetActorLocation)))) (LocalVariables|GetEnterLoc)) (Transformation|GetActorLocation))))) 2.0) (* (- 1.0 (Math|Float|Clamp(Float) (Class|KismetMathLibrary|InverseLerp 0.0 1.5e+02 (Math|Vector|VectorLength (- (+ (* ForwardVector (Math|Vector|VectorLength (- (LocalVariables|GetEnterLoc) (Transformation|GetActorLocation)))) (LocalVariables|GetEnterLoc)) (Transformation|GetActorLocation)))))) 2.0) (< (Math|Float|Clamp(Float) (Class|KismetMathLibrary|InverseLerp 0.0 1.5e+02 (Math|Vector|VectorLength (- (+ (* ForwardVector (Math|Vector|VectorLength (- (LocalVariables|GetEnterLoc) (Transformation|GetActorLocation)))) (LocalVariables|GetEnterLoc)) (Transformation|GetActorLocation))))) 0.5))) (> (Math|Vector|VectorLength (- (+ (* (LocalVariables|GetUpVec) 1e+02) (LocalVariables|GetEnterLoc)) _returnvalue)) (Math|Vector|VectorLength (- (+ (* (LocalVariables|GetUpVec) -1e+02) (LocalVariables|GetEnterLoc)) _returnvalue))))))) 5e+02) (LocalVariables|GetEnterLoc)))))