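; Prop_Destructible is a prop actor that loses Health when it takes damage and breaks apart once Health reaches zero or below.
; On death it disables collision on both StaticMesh and Destructible components, then enables physics simulation on the Destructible.
; It applies radius damage with an impulse to the Destructible at the actor's location to trigger the fracture.
; A short life span then removes the actor.
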(event Custom|TakeDamage
  (params (Damage :type Integer))
  (bind _destructible (Variables|Default|GetDestructible))
  (Variables|Default|SetHealth (- (Variables|Default|GetHealth) Damage))
  (if (<= (Variables|Default|GetHealth) 0)
    (Collision|SetCollisionEnabled (Variables|Default|GetStaticMesh) "NoCollision")
    (Collision|SetCollisionEnabled _destructible "NoCollision")
    (Physics|SetSimulatePhysics _destructible true)
    (Class|DestructibleComponent|ApplyRadiusDamage _destructible 1.0 (Transformation|GetActorLocation) 1e+02 1e+04 true)
    (Actor|SetLifeSpan 3.0)))

(event EventBeginPlay)

(event EventActorBeginOverlap
  (params (OtherActor :type Actor%20Object%20Reference)))

(event EventTick
  (params (DeltaSeconds :type Float%20%28single-precision%29)))

(fn ConstructionScript)