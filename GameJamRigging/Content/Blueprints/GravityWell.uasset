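; Gravity well actor that pulls first-person projectiles toward its center while they are inside its sphere.
; Sphere overlap events maintain a Projectiles array, adding only actors whose class exactly matches FirstPersonProjectile.
; Each tick applies a fixed-strength impulse toward the well to every tracked projectile's collision component, at the well's location, without distance falloff or delta-time scaling.
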(event OnComponentBeginOverlap(Sphere)
  (params (OtherActor :type Actor%20Object%20Reference) (OtherComp :type Primitive%20Component%20Object%20Reference) (OtherBodyIndex :type Integer) (bFromSweep :type Boolean) (SweepResult :type Hit%20Result%20Structure%20%28by%20ref%29))
  (if (== (Utilities|GetClass OtherActor) "/Game/Blueprints/FirstPersonProjectile.FirstPersonProjectile_C")
    (Utilities|Array|Add (Variables|Default|GetProjectiles) OtherActor)))

(event OnComponentEndOverlap(Sphere)
  (params (OtherActor :type Actor%20Object%20Reference) (OtherComp :type Primitive%20Component%20Object%20Reference) (OtherBodyIndex :type Integer))
  (Utilities|Array|RemoveItem (Variables|Default|GetProjectiles) OtherActor))

(event EventTick
  (params (DeltaSeconds :type Float%20%28single-precision%29))
  (bind _returnvalue (Transformation|GetActorLocation))
  (for _array_element (Variables|Default|GetProjectiles)
    (bind _asfirst_person_projectile (Utilities|Casting|CastToFirstPersonProjectile _array_element))
    (Physics|AddImpulseatLocation (Variables|/Game/Blueprints/FirstPersonProjectile.FirstPersonProjectile_C|GetCollisionComponent _asfirst_person_projectile) (* (Math|Vector|Normalize (- _returnvalue (Transformation|GetActorLocation _asfirst_person_projectile))) 5e+03) _returnvalue "None")))

(fn ConstructionScript)